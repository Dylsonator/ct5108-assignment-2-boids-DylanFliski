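; Player character that feeds mouse input to the BoidManager and lets the player place objects in the world.
; Every tick, a camera-channel trace from the cursor writes the hit point to the manager, alongside left and right button held states.
; Keys spawn cubes or rectangles at that point, raised to avoid clipping, and track them in a list that another key destroys.
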(event EventBeginPlay
  ;[1 1 1] Setting up manager & Spawn Locations for objects
  (bind _returnvalue (Actor|GetActorOfClass "/Script/Boids.BoidManager"))
  (Variables|Default|SetBoidManager _returnvalue))

(event EventTick
  (params (DeltaSeconds :type Float%20%28single-precision%29))
  (bind _returnvalue (Game|GetPlayerController 0))
  (bind (_worldlocation _worlddirection) (Game|Player|ConvertMouseLocationToWorldSpace _returnvalue))
  ;[1 1 1] Gets mouse position in world and sets it to the boid manager
  (bind _outhit (Collision|LineTraceByChannel _worldlocation (+ _worldlocation (* _worlddirection 5e+03)) "TraceTypeQuery2" false 0 "None"))
  (Variables|/Script/Boids.BoidManager|SetMousePosition (Variables|Default|GetBoidManager) (.impactpoint _outhit))
  (Variables|Default|SetRectangle%20Vector (Math|Vector|MakeVector (.x (Variables|/Script/Boids.BoidManager|GetMousePosition (Variables|Default|GetBoidManager))) (.y (Variables|/Script/Boids.BoidManager|GetMousePosition (Variables|Default|GetBoidManager))) (+ (.z (Variables|/Script/Boids.BoidManager|GetMousePosition (Variables|Default|GetBoidManager))) 1e+02)))
  (Variables|Default|SetCubeVector (Math|Vector|MakeVector (.x (Variables|/Script/Boids.BoidManager|GetMousePosition (Variables|Default|GetBoidManager))) (.y (Variables|/Script/Boids.BoidManager|GetMousePosition (Variables|Default|GetBoidManager))) (+ (.z (Variables|/Script/Boids.BoidManager|GetMousePosition (Variables|Default|GetBoidManager))) 5.0))))

(event Input|MouseEvents|LeftMouseButton
  (params (Key :type Key%20Structure :default "None"))
  (bind _boidmanager (Variables|Default|GetBoidManager))
  ;[1 1 1] Clicking logic (if pressed true, if released false)
  (:Pressed
    (bind _output_get (Variables|Default|SetIsPressed? true))
    (Variables|/Script/Boids.BoidManager|SetLeftIsPressed _boidmanager _output_get))
  (:Released
    (bind _output_get_2 (Variables|Default|SetIsPressed? false))
    (Variables|/Script/Boids.BoidManager|SetLeftIsPressed _boidmanager _output_get_2)))

(event Input|MouseEvents|RightMouseButton
  (params (Key :type Key%20Structure :default "None"))
  (bind _boidmanager (Variables|Default|GetBoidManager))
  ;[1 1 1] Clicking logic (if pressed true, if released false)
  (:Pressed
    (bind _output_get (Variables|Default|SetIsPressed? true))
    (Variables|/Script/Boids.BoidManager|SetRightIsPressed _boidmanager _output_get))
  (:Released
    (bind _output_get_2 (Variables|Default|SetIsPressed? false))
    (Variables|/Script/Boids.BoidManager|SetRightIsPressed _boidmanager _output_get_2)))

(event Input|KeyboardEvents|1
  (params (Key :type Key%20Structure :default "None"))
  ;[1 1 1] Spawn Objects
  (:Released
    (bind _returnvalue (Game|SpawnActorfromClass "/Game/Blueprints/Cube.Cube_C" (Math|Transform|MakeTransform (Variables|Default|GetCubeVector) "0, 0, 0" "1.000000,1.000000,1.000000") "AdjustIfPossibleButAlwaysSpawn" "MultiplyWithRoot" 0 0))
    (Utilities|Array|Add (Variables|Default|GetObjectList) _returnvalue)))

(event Input|KeyboardEvents|2
  (params (Key :type Key%20Structure :default "None"))
  ;[1 1 1] Spawn Objects
  (:Released
    (bind _returnvalue (Game|SpawnActorfromClass "/Game/Blueprints/Rectangle.Rectangle_C" (Math|Transform|MakeTransform (Variables|Default|GetRectangle%20Vector) "0, 0, 0" "1.000000,1.000000,1.000000") "AdjustIfPossibleButAlwaysSpawn" "MultiplyWithRoot" 0 0))
    (Utilities|Array|Add (Variables|Default|GetObjectList) _returnvalue)))

(event Input|KeyboardEvents|3
  (params (Key :type Key%20Structure :default "None"))
  ;[1 1 1] Spawn Objects
  (:Released
    (for _array_element (Variables|Default|GetObjectList)
      (Actor|DestroyActor _array_element))))

(fn ConstructionScript)